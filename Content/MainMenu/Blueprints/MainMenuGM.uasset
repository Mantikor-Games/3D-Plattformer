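; Main menu game mode for a 3D platformer that switches between the main, options, singleplayer savegame and quit screens.
; On BeginPlay it caches the game instance and shows the main menu; each screen is created once, given a reference to the game mode, then reused.
; Screen switches clear all widgets first, except the quit prompt, which is added on top.
; The savegame screen fills its list with save names from the game instance.
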(event `Savegamelist`
  (bind _list (`/Game/SavegameAndGameinstance/3D-PlattformerInstance.GiveSavegameNameList` (`self.Gameinstance`)))
  (bind _output_get (set `self.SavegameNames` _list))
  (`/Game/MainMenu/UI/SingleplayerSavegameUI.FillSavegameList` (`self.SingleplayerSavegameUI`) _output_get))

(event `self.ReceiveBeginPlay`
  (bind _as3d_plattformer_instance (cast `/Game/SavegameAndGameinstance/3D-PlattformerInstance` (`GameplayStatics.GetGameInstance`)))
  (set `self.Gameinstance` _as3d_plattformer_instance)
  (`self.ShowMainMenu`))

(event `ShowMainMenu`
  ;[1 1 1] Show Main Menu on Screen
  (`WidgetLayoutLibrary.RemoveAllWidgets`)
  (`/Engine/EditorBlueprintResources/StandardMacros.IsValid` (`self.MainMenuUI`)
    (:`Is Valid`
      _)
    (:`Is Not Valid`
      (bind _returnvalue (`|CreateWidget` "/Game/MainMenu/UI/MainMenuUI.MainMenuUI_C" (`GameplayStatics.GetPlayerController` 0) self))
      (set `self.MainMenuUI` _returnvalue)))
  (`UserWidget.AddToViewport` (`self.MainMenuUI`) 0))

(event `ShowOptions`
  ;[1 1 1] Show Options Menu on Screen
  (`WidgetLayoutLibrary.RemoveAllWidgets`)
  (`/Engine/EditorBlueprintResources/StandardMacros.IsValid` (`self.OptionsMenuUI`)
    (:`Is Valid`
      _)
    (:`Is Not Valid`
      (bind _returnvalue (`|CreateWidget` "/Game/MainMenu/UI/OptionsMenuUI.OptionsMenuUI_C" (`GameplayStatics.GetPlayerController` 0) self))
      (set `self.OptionsMenuUI` _returnvalue)))
  (`UserWidget.AddToViewport` (`self.OptionsMenuUI`) 0))

(event `ShowSingleplayerSaveGameUI`
  ;[1 1 1] Show Singleplayer Savegame UI on Screen
  (`WidgetLayoutLibrary.RemoveAllWidgets`)
  (`/Engine/EditorBlueprintResources/StandardMacros.IsValid` (`self.SingleplayerSavegameUI`)
    (:`Is Valid`
      _)
    (:`Is Not Valid`
      (bind _returnvalue (`|CreateWidget` "/Game/MainMenu/UI/SingleplayerSavegameUI.SingleplayerSavegameUI_C" (`GameplayStatics.GetPlayerController` 0) self))
      (set `self.SingleplayerSavegameUI` _returnvalue)))
  (`UserWidget.AddToViewport` (`self.SingleplayerSavegameUI`) 0)
  (`self.Savegamelist`))

(event `Quit Game`
  ;[1 1 1] Quitting the Game
  (`KismetSystemLibrary.QuitGame` (`GameplayStatics.GetPlayerController` 0) "Quit"))

(event `ShowQuitGameUI`
  ;[1 1 1] Show Quit Game UI on Screen
  (`/Engine/EditorBlueprintResources/StandardMacros.IsValid` (`self.QuitGameUI`)
    (:`Is Valid`
      _)
    (:`Is Not Valid`
      (bind _returnvalue (`|CreateWidget` "/Game/MainMenu/UI/QuitGameUI.QuitGameUI_C" (`GameplayStatics.GetPlayerController` 0) self))
      (set `self.QuitGameUI` _returnvalue)))
  (`UserWidget.AddToViewport` (`self.QuitGameUI`) 0))

(fn `UserConstructionScript`)